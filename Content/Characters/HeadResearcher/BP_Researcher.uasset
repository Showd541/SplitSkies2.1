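; BP_Researcher is the Head Researcher character, which shows a random line of advice in an on-screen talk widget.
; The Advice event creates a BP_Talk widget if none is valid, then sets its text from one of four Dialogue entries.
; Unconnected drafts cover messaging overlapping BPI_Interface actors and removing the widget after a delay.
; An author note says the logic still needs moving into the Ninja character to work.
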(event `Key|Tab`
  (params (Key :type "Key Structure"))
  ;[1 1 1] This needs to all be moved into the Ninja Character somewhere for this to work. Also add the BPI_Interface to the interface menu in the NinjaBP's Class Settings
)

(event `/Game/Characters/HeadResearcher/Interact/BPI_Interface.Advice`
  (`self.UI`
    (:`then`
      _)
    (:`else`
      (bind _returnvalue (`|CreateWidget` "/Game/Characters/HeadResearcher/Interact/BP_Talk.BP_Talk_C" (`GameplayStatics.GetPlayerController` 0)))
      (bind _output_get (set `self.UI` _returnvalue))
      (`UserWidget.AddToViewport` _output_get 0)))
  (`TextBlock.SetText` (`/Game/Characters/HeadResearcher/Interact/BP_Talk.TalkText` (`self.UI`)) (`KismetTextLibrary.Conv_StringToText` (`|GetArrayItem` (`self.Dialogue`) (`KismetMathLibrary.RandomInteger` 4)))))

(fn `UserConstructionScript`)