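; BP_DepthRecorder is a depth recorder prop among the Laputa equipment, animated with continuously spinning counter dials.
; Tick rolls nine dial components by DeltaSeconds, each ten times faster than the last, like geared odometer wheels.
; The rotation is purely time-driven and reads no actual depth value.
; Two unconnected experiments for bobbing the DepthBuoy, one using Sin and one a FlipFlop, never run.
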(event `self.ReceiveTick`
  (params (DeltaSeconds :type "Float (single-precision)"))
  (`SceneComponent.K2_AddRelativeRotation` (`self.Dial9`) (`KismetMathLibrary.MakeRotator` (* DeltaSeconds -200000000.0)) false false)
  (`SceneComponent.K2_AddRelativeRotation` (`self.Dial8`) (`KismetMathLibrary.MakeRotator` (* DeltaSeconds -20000000.0)) false false)
  (`SceneComponent.K2_AddRelativeRotation` (`self.Dial7`) (`KismetMathLibrary.MakeRotator` (* DeltaSeconds -2000000.0)) false false)
  (`SceneComponent.K2_AddRelativeRotation` (`self.Dial6`) (`KismetMathLibrary.MakeRotator` (* DeltaSeconds -200000.0)) false false)
  (`SceneComponent.K2_AddRelativeRotation` (`self.Dial5`) (`KismetMathLibrary.MakeRotator` (* DeltaSeconds -20000.0)) false false)
  (`SceneComponent.K2_AddRelativeRotation` (`self.Dial4`) (`KismetMathLibrary.MakeRotator` (* DeltaSeconds -2000.0)) false false)
  (`SceneComponent.K2_AddRelativeRotation` (`self.Dial3`) (`KismetMathLibrary.MakeRotator` (* DeltaSeconds -200.0)) false false)
  (`SceneComponent.K2_AddRelativeRotation` (`self.Dial2`) (`KismetMathLibrary.MakeRotator` (* DeltaSeconds -20.0)) false false)
  (`SceneComponent.K2_AddRelativeRotation` (`self.Dial`) (`KismetMathLibrary.MakeRotator` (* DeltaSeconds -2.0)) false false))

(fn `UserConstructionScript`)