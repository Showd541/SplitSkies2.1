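; BP_TextToTranslate is a world text display that shows a sentence in a symbol font, apparently for a language translation mechanic.
; On BeginPlay it uses WallNumber as an index into the DT_AllSentences row names to fetch that wall's sentence.
; It writes the row's Symbols, stripped of periods, into its WBP_MasterTextContainer widget and switches to the Splitskies font, keeping the other font settings.
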(event `self.ReceiveBeginPlay`
  (bind _outrownames (`DataTableFunctionLibrary.GetDataTableRowNames` "/Game/Language/InGameText/DT_AllSentences.DT_AllSentences"))
  (bind _returnvalue (`|GetDataTableRow` "/Game/Language/InGameText/DT_AllSentences.DT_AllSentences" (`|GetArrayItem` _outrownames (`self.WallNumber`)))
    (:`then`
      (bind _aswbp_master_text_container (cast `/Game/Language/UI/WBP_MasterTextContainer` (`WidgetComponent.GetUserWidgetObject` (`self.Widget`))))
      (bind _textblock (`/Game/Language/UI/WBP_MasterTextContainer.TextBlock` _aswbp_master_text_container))
      (`TextBlock.SetText` _textblock (`KismetTextLibrary.Conv_StringToText` (`KismetStringLibrary.Replace` (`KismetTextLibrary.Conv_TextToString` (`.Symbols_4_17255F1741B75211355D8DAEFEBE3791` (break `/Game/Language/InGameText/S_AllText` _returnvalue))) "." "  ")))
      (bind (_font_fontobject _font_fontmaterial _font_outlinesettings _font_typefacefontname _font_size _font_letterspacing) (break `SlateFontInfo` (`TextBlock.Font` _textblock)))
      (`TextBlock.SetFont` _textblock (make `SlateFontInfo` "/Game/Language/InGameText/Font/Splitskiesfinalfont-Regular_Font.Splitskiesfinalfont-Regular_Font" _font_fontmaterial _font_outlinesettings _font_typefacefontname _font_size _font_letterspacing)))
    (:`RowNotFound`
      (`KismetSystemLibrary.PrintString` "Row not found"))))

(fn `UserConstructionScript`)