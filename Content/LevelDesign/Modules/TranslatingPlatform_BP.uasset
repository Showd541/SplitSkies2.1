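; Moving platform Blueprint for level design that travels up and down along Z in an endless loop while rotating.
; From BeginPlay, two eased, timed MoveComponentTo calls move the root by RelativeZMoveTo and back, swinging it between two fixed rotations with a short pause after each move.
; Each target is offset from the actor's current location when the move begins, rather than from a stored start position.
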(event `self.ReceiveBeginPlay`
  (`KismetSystemLibrary.MoveComponentTo` (`self.DefaultSceneRoot`) (+ (`self.K2_GetActorLocation`) (`KismetMathLibrary.MakeVector` 0.0 0.0 (`self.RelativeZMoveTo`))) (struct :`Yaw` 90.0 :`Roll` 90.0) true true 4.0 :!label _label)
  (`KismetSystemLibrary.Delay` 1.0)
  (`KismetSystemLibrary.MoveComponentTo` (`self.DefaultSceneRoot`) (+ (`self.K2_GetActorLocation`) (`KismetMathLibrary.MakeVector` 0.0 0.0 (* (`self.RelativeZMoveTo`) -1.0))) (struct :`Yaw` -90.0) true true 4.0)
  (`KismetSystemLibrary.Delay` 1.0)
  (goto _label))

(fn `UserConstructionScript`)